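; Interactable button that, when triggered, notifies the first BP_ChangingNumberManager found in the level via OnActivation.
; OnInteract also restarts a Niagara effect, animates the button with a timeline offset scaled by the base's world scale, and plays FMOD audio.
; The incoming Speed value drives the sound's Repetitions parameter.
; Tick turns the Niagara effect toward the player pawn in yaw and roll, keeping the root's pitch.
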(event Custom|Audio%20Behaviour
  (params (Pitch :type Float%20%28double-precision%29))
  ;[1 1 1] Audio
  (Class|FMODAudioComponent|SetParameter (Variables|Default|GetFMODAudio) "Repetitions" (* (- Pitch 1.0) 1.1))
  (Class|FMODAudioComponent|Release (Variables|Default|GetFMODAudio))
  (Class|FMODAudioComponent|Play (Variables|Default|GetFMODAudio)))

(event Custom|Button%20Animation
  ;[1 1 1] Animation
  (bind _button_down_ (Timeline|Timeline PlayFromStart)
    (:Update
      (Transformation|SetRelativeLocation (Variables|Default|GetButton) (Math|Vector|MakeVector 0.0 0.0 (+ (* _button_down_ (* 3e+03 (.z (Transformation|GetWorldScale (Variables|Default|GetSocle))))) (Variables|Default|GetStartLocation))) false false))))

(event EventBeginPlay
  (Variables|Default|SetStartLocation (.z (Variables|/Script/Engine.SceneComponent|GetRelativeLocation (Variables|Default|GetButton)))))

(event Collision|EventActorBeginOverlap
  (params (OtherActor :type Actor%20Object%20Reference)))

(event EventOnInteract
  (params (Speed :type Float%20%28double-precision%29))
  (CallFunction|AudioBehaviour Speed)
  (CallFunction|ButtonAnimation)
  (Components|Activation|Deactivate (Variables|Default|GetNiagara))
  (Components|Activation|Activate (Variables|Default|GetNiagara) false)
  (bind _outactors (Actor|GetAllActorsOfClass "/Game/Elknir/Blueprints/ChangingNumbers/BP_ChangingNumberManager.BP_ChangingNumberManager_C"))
  (Utilities|IsValid (Utilities|Array|Get(acopy) _outactors)
    (:Is%20Valid
      (Default|OnActivation (Utilities|Array|Get(acopy) _outactors)))))

(event EventTick
  (params (DeltaSeconds :type Float%20%28single-precision%29))
  (bind _returnvalue (Transformation|GetActorLocation))
  (bind _returnvalue_2 (Game|Player|GetPlayerPawn 0))
  (bind _returnvalue_3 (Transformation|GetActorLocation _returnvalue_2))
  (bind _returnvalue_4 (Math|Rotator|FindLookatRotation _returnvalue _returnvalue_3))
  ;[0.3438 0.3438 0.3438] Niagara System facing camera
  ; Maybe baking the particule system?
  (Transformation|SetWorldRotation (Variables|Default|GetNiagara) (Math|Rotator|MakeRotator (.roll _returnvalue_4) (.pitch (Transformation|GetWorldRotation (Variables|Default|GetDefaultSceneRoot))) (- (.yaw _returnvalue_4) 1.8e+02)) false false))

(fn ConstructionScript)