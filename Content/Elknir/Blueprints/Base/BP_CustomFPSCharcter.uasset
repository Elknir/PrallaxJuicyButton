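; First-person character Blueprint that adds a press interaction, with a pressing animation that speeds up when spammed.
; IA_Interact plays AM_Pressing behind a DoOnce gate; its "canInteract" notify reopens the gate early, raises the clamped play rate and switches to the "Spam" section.
; The "Pressed" notify sphere-traces ahead of the camera and sends the current play rate to BPI_Interactibles actors.
; Montage completion resets rate and section.
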(event Custom|Interactible%20Detection
  (bind _firstpersoncamera (Variables|Default|GetFirstPersonCamera))
  (bind _returnvalue (Transformation|GetWorldLocation _firstpersoncamera))
  (bind _returnvalue_2 (Math|Vector|GetForwardVector _firstpersoncamera))
  (bind _returnvalue_3 (* _returnvalue_2 5e+01))
  ;[1 1 1] Forward Detection
  (bind _outhit (Collision|SphereTraceByChannel (+ _returnvalue _returnvalue_3) (+ _returnvalue (* _returnvalue_3 1.5)) 3e+01 "TraceTypeQuery1" false 0 "None" true "(R=1.000000,G=0.000000,B=0.000000,A=1.000000)" "(R=0.000000,G=1.000000,B=0.000000,A=1.000000)" 2.0))
  ;[1 1 1] Interactible activation
  (if (Utilities|DoesObjectImplementInterface (.hitactor _outhit) "/Game/Elknir/Blueprints/Interactibles/BPI_Interactibles.BPI_Interactibles_C")
    (Class|BPIInteractibles|OnInteract(Message) (.hitactor _outhit) (Variables|Default|GetCurrrent%20Pressing%20Play%20Rate))))

(event Custom|Reset%20Interact
  (Utilities|FlowControl|DoOnce false) ; enters at Reset
)

(event Input|EnhancedActionEvents|EnhancedInputActionIA_Interact
  (params (ActionValue :type Boolean) (ElapsedSeconds :type Float%20%28double-precision%29) (TriggeredSeconds :type Float%20%28double-precision%29) (InputAction :type Input%20Action%20Object%20Reference :default "/Game/Elknir/Blueprints/Inputs/IA_Interact.IA_Interact"))
  (Utilities|FlowControl|DoOnce false
    (:Completed
      (bind _notifyname (Animation|Montage|PlayMontage (Variables|Default|GetFirstPersonMesh) "/Game/Elknir/Animations/AM_Pressing.AM_Pressing" (Variables|Default|GetCurrrent%20Pressing%20Play%20Rate) 0.0 (Variables|Default|GetStarting%20Point%20Animation))
        (:OnCompleted
          (CallFunction|ResetInteract)
          (Variables|Default|SetCurrrent%20Pressing%20Play%20Rate (Variables|Default|GetBase%20Pressing%20Play%20Rate))
          (Variables|Default|SetStarting%20Point%20Animation "None"))
        (:OnNotifyBegin
          (Utilities|FlowControl|Sequence
            (:then_0
              (if (== _notifyname "Pressed")
                (CallFunction|InteractibleDetection)))
            (:then_1
              (if (== _notifyname "canInteract")
                (CallFunction|ResetInteract)
                (Variables|Default|SetCurrrent%20Pressing%20Play%20Rate (Math|Float|Clamp(Float) (+ (Variables|Default|GetCurrrent%20Pressing%20Play%20Rate) 0.1) 1.0 1.7))
                (Variables|Default|SetStarting%20Point%20Animation "Spam")))))))))

(event EventBeginPlay
  (Variables|Default|SetCurrrent%20Pressing%20Play%20Rate (Variables|Default|GetBase%20Pressing%20Play%20Rate)))

(event Collision|EventActorBeginOverlap
  (params (OtherActor :type Actor%20Object%20Reference)))

(event EventTick
  (params (DeltaSeconds :type Float%20%28single-precision%29)))

(fn ConstructionScript
  (|CallParentFunction))