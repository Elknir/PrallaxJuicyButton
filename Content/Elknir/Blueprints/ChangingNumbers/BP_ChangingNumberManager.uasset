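; Slot-machine style manager that spawns a row of BP_ChangingNumber actors on BeginPlay and turns their stopped digits into a money reward.
; Each activation locks the next number in sequence, using a modulo counter to detect when all are locked.
; It then combines the digits by powers of ten, passes the value to BP_MoneyRain's effect, and unlocks all after a short delay, ignoring activations meanwhile.
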(event Custom|OnActivation
  (if (not (Variables|Default|GetIsReseting))
    (CallFunction|StopDigits)
    (if (== (Variables|ChangingNumbers|GetTargeted%20Number%20Of%20Changing%20Numbers) 0)
      (Variables|Default|SetIsReseting true)
      (CallFunction|RewardPlayer)
      (Utilities|FlowControl|Delay 0.5)
      (CallFunction|UnlockAllDigits)
      (Variables|Default|SetIsReseting false))))

(event Custom|Stop%20Digits
  (Default|LockNumber (Utilities|Array|Get(acopy) (Variables|ChangingNumbers|GetAllChangingNumbers) (Variables|ChangingNumbers|GetTargeted%20Number%20Of%20Changing%20Numbers)))
  (bind _result (Math|Integer|IncrementInt (Variables|ChangingNumbers|GetTargeted%20Number%20Of%20Changing%20Numbers))
    (:%20%20
      (Variables|ChangingNumbers|SetTargeted%20Number%20Of%20Changing%20Numbers (Math|Integer|%(Integer) _result (Variables|ChangingNumbers|GetNumber%20Of%20Changing%20Numbers))))))

(event Custom|Unlock%20All%20Digits
  (for _array_element (Variables|ChangingNumbers|GetAllChangingNumbers)
    (Default|UnlockNumber _array_element)))

(event Custom|Activate%20Money%20VFX
  (params (Reward%20Value :type Integer))
  ;[1 0.01524 0] TODO : Make an interface
  (bind _returnvalue (Actor|GetActorOfClass "/Game/Elknir/Blueprints/ChangingNumbers/BP_MoneyRain.BP_MoneyRain_C"))
  (Utilities|IsValid _returnvalue
    (:Is%20Valid
      (Default|ActivateEffect _returnvalue Reward%20Value))))

(event Custom|Reward%20Player
  (bind _found_value (CallFunction|FindRewardInt))
  (CallFunction|ActivateMoneyVFX _found_value))

(event EventBeginPlay
  (bind _returnvalue (Transformation|GetActorTransform))
  (for _index (range 0 (- (Variables|ChangingNumbers|GetNumber%20Of%20Changing%20Numbers) 1))
    (bind _returnvalue_2 (Game|SpawnActorfromClass "/Game/Elknir/Blueprints/ChangingNumbers/BP_ChangingNumber.BP_ChangingNumber_C" (Math|Transform|MakeTransform (+ (.location _returnvalue) (Math|Vector|MakeVector 0.0 (* (* _index (Variables|ChangingNumbers|GetSpacing%20Between%20Numbers)) -1.0) 0.0)) (.rotation _returnvalue) (.scale _returnvalue)) "Undefined" "MultiplyWithRoot" 0 0))
    (Utilities|Array|AddUnique (Variables|ChangingNumbers|GetAllChangingNumbers) _returnvalue_2)))

(fn ConstructionScript
  (Utilities|Array|Clear (Variables|ChangingNumbers|GetAllChangingNumbers)))

(fn FindRewardInt
  (LocalVariables|SetReward%20Value 0)
  (for (_array_element _array_index) (Variables|ChangingNumbers|GetAllChangingNumbers)
    (bind _selected_digit (Default|GetSelectedDigit _array_element))
    (LocalVariables|SetReward%20Value (+ (* _selected_digit (Math|Float|Truncate (Math|Float|Power 1e+01 (Math|Conversions|ToFloat(Integer) _array_index)))) (LocalVariables|GetReward%20Value))))
  (return (LocalVariables|GetReward%20Value)))