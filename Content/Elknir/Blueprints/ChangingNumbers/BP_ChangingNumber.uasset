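; Actor that displays a changing digit through a widget component, with controls to lock it and read its value.
; The WBPChangingInt widget is assigned in the construction script and again on BeginPlay to keep the reference.
; LockNumber sets the widget's locked flag, while UnlockNumber clears it and sets a random digit from 0 to 8.
; GetSelectedDigit returns the widget's current digit.
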(event Custom|Lock%20Number
  (Variables|/Game/Elknir/Blueprints/ChangingNumbers/WBP_ChangingNumber.WBP_ChangingNumber_C|SetIs%20Digit%20Locked (Variables|Default|GetWBP_ChangingInt) true))

(event Custom|Unlock%20Number
  (bind _wbp_changingint (Variables|Default|GetWBP_ChangingInt))
  (Variables|/Game/Elknir/Blueprints/ChangingNumbers/WBP_ChangingNumber.WBP_ChangingNumber_C|SetIs%20Digit%20Locked _wbp_changingint false)
  (Default|SetDigitText _wbp_changingint (Math|Random|RandomInteger 9)))

(event EventBeginPlay
  ;[1 1 1] Must put it or I lose the reference
  (UserInterface|SetWidget (Variables|Default|GetWidget) (Variables|Default|GetWBP_ChangingInt)))

(event Collision|EventActorBeginOverlap
  (params (OtherActor :type Actor%20Object%20Reference)))

(event EventTick
  (params (DeltaSeconds :type Float%20%28single-precision%29)))

(fn ConstructionScript
  (UserInterface|SetWidget (Variables|Default|GetWidget) (Variables|Default|GetWBP_ChangingInt)))

(fn GetSelectedDigit
  (return (Variables|/Game/Elknir/Blueprints/ChangingNumbers/WBP_ChangingNumber.WBP_ChangingNumber_C|GetCurrent%20Digit (Variables|Default|GetWBP_ChangingInt))))