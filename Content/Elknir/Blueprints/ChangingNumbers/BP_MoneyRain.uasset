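; BP_MoneyRain is an effect actor that plays a Niagara money rain when a reward is given.
; ActivateEffect restarts the Niagara component and sets its SpawnRate from the reward value, clamped between zero and CoinLimit.
; It also fixes the loop duration, so larger rewards yield denser bursts up to the cap.
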(event Custom|Activate%20Effect
  (params (Reward%20Value :type Integer))
  (Components|Activation|Deactivate (Variables|Default|GetNiagara))
  (Components|Activation|Activate (Variables|Default|GetNiagara) false)
  (Niagara|SetNiagaraVariable(Float) (Variables|Default|GetNiagara) "SpawnRate" (Math|Conversions|ToFloat(Integer) (Math|Integer|Clamp(Integer) Reward%20Value 0 (Variables|Default|GetCoin%20Limit))))
  (Niagara|SetNiagaraVariable(Float) (Variables|Default|GetNiagara) "Loop Duration" 1.0))

(event EventBeginPlay)

(event Collision|EventActorBeginOverlap
  (params (OtherActor :type Actor%20Object%20Reference)))

(event EventTick
  (params (DeltaSeconds :type Float%20%28single-precision%29)))

(fn ConstructionScript)